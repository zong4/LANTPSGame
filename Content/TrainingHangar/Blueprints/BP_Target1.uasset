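; BP_Target1 is a shootable moving target in the training hangar, with a cart that slides along X.
; On BeginPlay the server randomly picks one of three timelines, which Tick plays to drive the cart.
; When IsShoted is set through SetIsShoted, the server's Tick stops that timeline and pitches the physics constraint to -90 degrees.
; The OnRep functions for IsShoted and TimelineIndex are empty.
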(event `self.ReceiveBeginPlay`
  (`/Engine/EditorBlueprintResources/ActorMacros.Switch Has Authority`
    (:`Authority`
      (set `self.TimelineIndex` (`KismetMathLibrary.RandomInteger` 3)))))

(event `self.ReceiveTick`
  (params (DeltaSeconds :type "Float (single-precision)"))
  (bind _sm_cart (`self.SM_Cart`))
  (bind _timelineindex (`self.TimelineIndex`))
  (`/Engine/EditorBlueprintResources/ActorMacros.Switch Has Authority`
    (:`Authority`
      (if (`self.IsShoted`)
        (`SceneComponent.K2_SetRelativeRotation` (`self.PhysicsConstraint`) (struct :`Roll` -90.0) false false)
        (switch `int` _timelineindex
          (:`0`
            (bind (_direction _float) (`Timeline|Timeline` :`NewTime` 1.0 :!via `Stop` :!label _label)
              (:`Update`
                (`SceneComponent.K2_SetRelativeLocation` _sm_cart (`KismetMathLibrary.MakeVector` _float) false false))))
          (:`1`
            (bind (_direction_2 _float_2) (`Timeline|时间轴_0` :`NewTime` 1.0 :!via `Stop` :!label _label_2)
              (:`Update`
                (`SceneComponent.K2_SetRelativeLocation` _sm_cart (`KismetMathLibrary.MakeVector` _float_2) false false))))
          (:`2`
            (bind (_direction_3 _float_3) (`Timeline|时间轴_1` :`NewTime` 1.0 :!via `Stop` :!label _label_3)
              (:`Update`
                (`SceneComponent.K2_SetRelativeLocation` _sm_cart (`KismetMathLibrary.MakeVector` _float_3) false false)))))
        (else
          (switch `int` _timelineindex
            (:`0`
              (goto _label))
            (:`1`
              (goto _label_2))
            (:`2`
              (goto _label_3))))))))

(event `EVESetIsShoted`
  (params (IsShoted :type Boolean))
  (set `self.IsShoted` IsShoted))

(fn `OnRep_IsShoted`)

(fn `OnRep_TimelineIndex`)

(fn `SetIsShoted`
  (params (IsShoted :type Boolean))
  (`self.EVESetIsShoted` IsShoted))

(fn `UserConstructionScript`)